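; BP_Bottle is an interactable bottle actor whose mesh can be shown or hidden and which opens a typing screen.
; SetVisible and OffVisible events call helper functions that toggle the BottleMesh visibility.
; Interact creates a TypingWidget, adds it to the viewport, switches the player to UI-only input and shows the mouse cursor.
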(event Custom|SetVisible
  (CallFunction|SetVisibility))

(event Custom|OffVisible
  (CallFunction|OffVisibiluty))

(event EventBeginPlay)

(event Collision|EventActorBeginOverlap
  (params (OtherActor :type Actor%20Object%20Reference)))

(event EventTick
  (params (DeltaSeconds :type Float%20%28single-precision%29)))

(event EventInteract
  (params (Interactor :type Actor%20Object%20Reference))
  (bind _returnvalue (Game|GetPlayerController 0))
  (bind _returnvalue_2 (UserInterface|CreateWidget "/Game/WidgetBP/TypingWidget.TypingWidget_C"))
  (UserInterface|Viewport|AddtoViewport _returnvalue_2 0)
  (Input|SetInputModeUIOnly _returnvalue 0 "DoNotLock" true)
  (Variables|/Script/Engine.PlayerController|SetbShowMouseCursor _returnvalue true))

(fn ConstructionScript)

(fn SetVisibility
  (Rendering|SetVisibility (Variables|Default|GetBottleMesh) true false))

(fn OffVisibiluty
  (Rendering|SetVisibility (Variables|Default|GetBottleMesh) false false))